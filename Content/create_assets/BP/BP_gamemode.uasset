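; BP_gamemode is a game mode Blueprint that respawns the player character when it is destroyed.
; On BeginPlay it binds to the player pawn's OnDestroyed event.
; When that fires, it spawns a new BP_mainCharacter at the player start, has player controller 0 possess it, and rebinds to the new pawn so respawning repeats.
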(event Custom|RespawnEvent
  (Game|AssignOnDestroyed (Game|Player|GetPlayerPawn 0) (delegate Custom|RespawnCharacter)))

(event Custom|RespawnCharacter
  (params (DestroyedActor :type Actor%20Object%20Reference))
  (bind _returnvalue (Game|SpawnActorfromClass "/Game/create_assets/Player/BP_mainCharacter.BP_mainCharacter_C" (Transformation|GetActorTransform (Class|GameModeBase|FindPlayerStart)) "Undefined" 0 0))
  (Pawn|Possess (Game|GetPlayerController 0) _returnvalue)
  (CallFunction|RespawnEvent))

(event EventBeginPlay
  (CallFunction|RespawnEvent))

(event EventTick
  (params (DeltaSeconds :type Float%20%28single-precision%29)))

(fn ConstructionScript)