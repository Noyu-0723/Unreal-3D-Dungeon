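; BP_Door is a hinged door that the player opens and closes with the OpenDoor input while near it.
; Overlap of its Box by a ThirdPersonCharacter enables input and opens a Gate, and leaving disables input and closes it.
; Each press passing the Gate alternates via FlipFlop between playing and reversing the DoorAnimation timeline, which lerps the Door's yaw between CloseAngle and OpenAngle.
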(event OnComponentBeginOverlap(Box)
  (params (OverlappedComponent :type Primitive%20Component%20Object%20Reference) (OtherActor :type Actor%20Object%20Reference) (OtherComp :type Primitive%20Component%20Object%20Reference) (OtherBodyIndex :type Integer) (bFromSweep :type Boolean) (SweepResult :type Hit%20Result%20Structure%20%28by%20ref%29))
  (Utilities|Casting|CastToThirdPersonCharacter OtherActor)
  (Input|EnableInput (Game|GetPlayerController 0))
  (Utilities|FlowControl|Gate false) ; enters at Open
)

(event OnComponentEndOverlap(Box)
  (params (OverlappedComponent :type Primitive%20Component%20Object%20Reference) (OtherActor :type Actor%20Object%20Reference) (OtherComp :type Primitive%20Component%20Object%20Reference) (OtherBodyIndex :type Integer))
  (Utilities|Casting|CastToThirdPersonCharacter OtherActor)
  (Input|DisableInput (Game|GetPlayerController 0))
  (Utilities|FlowControl|Gate false) ; enters at Close
)

(event Input|ActionEvents|InputActionOpenDoor
  (params (Key :type Key%20Structure))
  (:Pressed
    (Utilities|FlowControl|Gate false
      (:Exit
        (Utilities|FlowControl|FlipFlop
          (:A
            (bind _door_track (Timeline|Door%20Animation Play)
              (:Update
                (Transformation|SetRelativeRotation (Variables|Default|GetDoor) (Math|Rotator|MakeRotator 0.0 0.0 (Math|Float|Lerp (Variables|Default|GetClose%20Angle) (Variables|Default|GetOpen%20Angle) _door_track)) false false))))
          (:B
            (Timeline|Door%20Animation Reverse)))))))

(fn ConstructionScript)